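; Stun skill pickup that gives the player a periodic stun against enemies.
; On overlap it notifies its chest, then either registers as the player's stun or, if one exists, raises its own StunAmount using a modulo and destroys itself.
; Once active, a Tick-driven seconds counter triggers StunEnemy at each SpellCountdown.
; It picks a random enemy and, unless tagged Stunned, plays zap effects and sends StunMessage.
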(event OnComponentBeginOverlap(StaticMesh)
  (params (OverlappedComponent :type Primitive%20Component%20Object%20Reference) (OtherActor :type Actor%20Object%20Reference) (OtherComp :type Primitive%20Component%20Object%20Reference) (OtherBodyIndex :type Integer) (bFromSweep :type Boolean) (SweepResult :type Hit%20Result%20Structure%20%28by%20ref%29))
  (bind _player (Variables|Default|GetPlayer))
  (Components|DestroyComponent (Variables|Default|GetStaticMesh))
  (Utilities|FlowControl|Delay 0.0)
  (bind _chest (Variables|Default|GetChest)
    (:then
      (Default|ChestDestroy _chest self))
    (:else
      _))
  (if (Variables|/Game/Blueprints/Characters/Player/BP_Player.BP_Player_C|GetHasStun (Variables|Default|GetPlayer))
    (Variables|Stun|SetStunAmount (+ (Variables|Stun|GetStunAmount) (Math|Float|%(Float) (Variables|Stun|GetStunAmount) (Variables|Stun|GetIncreaseStunPercentage))))
    (Actor|DestroyActor)
    (else
      (Variables|System|SetCanWork true)
      (Variables|/Game/Blueprints/Characters/Player/BP_Player.BP_Player_C|SetHasStun _player true)
      (Variables|/Game/Blueprints/Characters/Player/BP_Player.BP_Player_C|SetStun _player self))))

(event EventTick
  (params (DeltaSeconds :type Float%20%28single-precision%29))
  (CallFunction|CountSeconds DeltaSeconds)
  (if (and (== (Variables|System|GetCurrentTime) (Variables|Default|GetSpellCountdown)) (Variables|System|GetCanWork))
    (Variables|System|SetCurrentTime 0)
    (CallFunction|StunEnemy)))

(event EventBeginPlay
  (bind _asbp_player (Utilities|Casting|CastToBP_Player (Game|Player|GetPlayerPawn 0)))
  (Variables|Default|SetPlayer _asbp_player))

(fn ConstructionScript)

(fn CountSeconds
  (params (DeltaTİme :type Float%20%28double-precision%29))
  (bind _output_get (Variables|System|SetAccumulatedTime (+ DeltaTİme (Variables|System|GetAccumulatedTime))))
  (if (>= _output_get 1.0)
    (Variables|System|SetAccumulatedTime (- (Variables|System|GetAccumulatedTime) 1.0))
    (if (Variables|System|GetCanWork)
      (Math|Integer|IncrementInt (Variables|System|GetCurrentTime)
        (:%20%20
          _))
      (else
        (Variables|System|SetCurrentTime 0)))
    (return)))

(fn StunEnemy
  (bind _output_get (LocalVariables|SetMyTarget (.OutItem (Utilities|Array|Random (Variables|/Game/Blueprints/Characters/Player/BP_Player.BP_Player_C|GetEnemies (Variables|Default|GetPlayer))))))
  (Utilities|IsValid _output_get
    (:Is%20Valid
      (if (not (Actor|ActorHasTag (LocalVariables|GetMyTarget) "Stunned"))
        (Niagara|SpawnSystematLocation "/Game/Vefects/Zap_VFX/VFX/Zap/Particles/NS_Zap_03_Yellow.NS_Zap_03_Yellow" (Math|Vector|MakeVector (.x (Transformation|GetActorLocation (LocalVariables|GetMyTarget))) (.y (Transformation|GetActorLocation (LocalVariables|GetMyTarget))) (- (.z (Transformation|GetActorLocation (LocalVariables|GetMyTarget))) 9e+01)))
        (Audio|PlaySoundatLocation (Variables|Stun|GetStunSound) (Transformation|GetActorLocation (LocalVariables|GetMyTarget)) "0, 0, 0" 1.0 1.0 0.0 0 0 0 0)
        (Class|BPIMessager|Stun(Message) (LocalVariables|GetMyTarget) (Variables|Stun|GetStunAmount))
        (return)))))