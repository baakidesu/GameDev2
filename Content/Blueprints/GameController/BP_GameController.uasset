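; Game controller that spawns timed enemy waves around the player and periodically places chests.
; Tick drives a one-second counter that starts each wave at its mapped trigger time and flags chests on a cooldown for random TargetPoints.
; Per-wave maps set hardness and count, choosing random classes from the matching enemy array.
; Each wave shares one reachable navmesh spawn point, retried recursively when too close to the player.
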(event EventBeginPlay
  (bind _returnvalue (Actor|GetActorOfClass "/Game/Blueprints/Characters/Player/BP_Player.BP_Player_C"))
  (Variables|Player|SetPlayer _returnvalue)
  (bind _outactors (Actor|GetAllActorsOfClass "/Script/Engine.TargetPoint"))
  (Variables|Chest|SetChestPossibleLocationds _outactors))

(event EventDieMessagetoSpawner
  (bind _result (Math|Integer|DecrementInt (Variables|Wave|GetActiveEnemyCount))
    (:%20%20
      (if (== _result 0)
        _))))

(event EventTick
  (params (DeltaSeconds :type Float%20%28single-precision%29))
  (CallFunction|CountSeconds DeltaSeconds)
  (if (Variables|Chest|GetCanCreateChest)
    (CallFunction|CreateChest))
  (if (== (Variables|Default|GetCurrentTime) (.Value (Utilities|Map|Find (Variables|Wave|GetWaveTriggers) (Variables|Wave|GetCurrentWave))))
    (CallFunction|StartWave)))

(fn ConstructionScript)

(fn GetWaveHardnessandEnemyCount
  (params (Wave :type Integer%20%28by%20ref%29))
  (return (.Value (Utilities|Map|Find (Variables|Wave|GetWaveHardness) Wave)) (.Value (Utilities|Map|Find (Variables|Wave|GetWaveEnemyCount) Wave))))

(fn StartWave
  (bind _currentwave (Variables|Wave|GetCurrentWave))
  (bind (_hardness _enemycount) (CallFunction|GetWaveHardnessandEnemyCount _currentwave))
  (Development|PrintString (Utilities|String|Append "Starting Wave" (Utilities|String|ToString(Integer) (Variables|Wave|GetCurrentWave))))
  (bind _randomlocation (CallFunction|GetReachableTransform))
  (LocalVariables|SetRandomLoc _randomlocation)
  (switch Utilities|FlowControl|Switch|SwitchonEnum_Hardness _hardness
    (:NewEnumerator0
      (Development|PrintString "easy" true true "(R=0.000000,G=0.161832,B=1.000000,A=1.000000)")
      (CallFunction|SpawnEnemies _enemycount (Variables|EnemyTypes|GetEasyEnemies) (LocalVariables|GetRandomLoc)))
    (:NewEnumerator1
      (CallFunction|SpawnEnemies _enemycount (Variables|EnemyTypes|GetMediumEnemies) (LocalVariables|GetRandomLoc)))
    (:NewEnumerator2
      (Development|PrintString "hard" true true "(R=0.000000,G=0.161832,B=1.000000,A=1.000000)")
      (CallFunction|SpawnEnemies _enemycount (Variables|EnemyTypes|GetHardEnemies) (LocalVariables|GetRandomLoc))))
  (Math|Integer|IncrementInt (Variables|Wave|GetCurrentWave)))

(fn SpawnEnemies
  (params (EnemyCount :type Integer) (Array :type Array%20of%20BP%20Enemy%20Class%20References) (SpawnTransform :type Transform))
  (bind _outitem (Utilities|Array|Random Array))
  (Development|PrintString (Utilities|String|ToString(Integer) EnemyCount))
  (for _index (range 1 EnemyCount)
    (if (Utilities|IsValidClass _outitem)
      (bind _returnvalue (Game|SpawnActorfromClass _outitem SpawnTransform "AdjustIfPossibleButAlwaysSpawn" "MultiplyWithRoot" 0 0))
      (Utilities|IsValid _returnvalue
        (:Is%20Valid
          (Development|PrintString "YES")
          (Math|Integer|IncrementInt (Variables|Wave|GetActiveEnemyCount)))
        (:Is%20Not%20Valid
          (Development|PrintString "NO")))
      (else
        (return))))
  (return))

(fn CountSeconds
  (params (DeltaTime :type Float%20%28double-precision%29))
  (bind _output_get (Variables|Default|SetAccumulatedTime (+ DeltaTime (Variables|Default|GetAccumulatedTime))))
  (if (>= _output_get 1.0)
    (Variables|Default|SetAccumulatedTime (- (Variables|Default|GetAccumulatedTime) 1.0))
    (bind _result (Math|Integer|IncrementInt (Variables|Default|GetCurrentTime))
      (:%20%20
        (if (== (Math|Integer|%(Integer) _result (Variables|Chest|GetChestCooldown)) 0)
          (Variables|Chest|SetCanCreateChest true))
        (return)))))

(fn GetReachableTransform
  (bind _output_get (LocalVariables|SetPlayerLoc (Transformation|GetActorLocation (Variables|Player|GetPlayer))))
  (LocalVariables|SetRandomLoc (.RandomLocation (AI|Navigation|GetRandomReachablePointinRadius _output_get 4e+03 0 0)))
  (if (>= (Math|Vector|VectorLength (- (LocalVariables|GetPlayerLoc) (LocalVariables|GetRandomLoc))) (Variables|Player|GetMinDistanceToPlayer))
    (return (Math|Transform|MakeTransform (+ (LocalVariables|GetRandomLoc) "0.000000,0.000000,200.000000")))
    (else
      (CallFunction|GetReachableTransform))))

(fn CreateChest
  (Game|SpawnActorfromClass "/Game/Blueprints/Chest/BP_Chest.BP_Chest_C" (Math|Conversions|ToTransform(Vector) (Transformation|GetActorLocation (.OutItem (Utilities|Array|Random (Variables|Chest|GetChestPossibleLocationds))))) "Undefined" "MultiplyWithRoot" 0 0)
  (Variables|Chest|SetCanCreateChest false)
  (Audio|PlaySoundatLocation "/Game/Vefects/Zap_VFX/Audio/SFX_Vefects_Zap_Big_02_Cue.SFX_Vefects_Zap_Big_02_Cue" (Transformation|GetActorLocation (Variables|Player|GetPlayer)) "0, 0, 0" 1.0 1.0 0.0 0 0 0 0)
  (return))