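; BP_Enemy is an enemy that chases the player, takes damage and can be stunned.
; A looping timer started on BeginPlay periodically issues AI MoveTo toward the cached player pawn.
; HitDamage lowers Health and calls Die at zero, which notifies EnemySpawner and destroys the actor only if that spawner is valid.
; Stun disables movement for a given delay, then restores walking, with debug prints throughout.
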(event Custom|AIMove
  (AI|AIMoveTo self "0, 0, 0" (Variables|Default|GetAs%20BP%20Player) 5.0 false))

(event EventBeginPlay
  (bind _asbp_player (Utilities|Casting|CastToBP_Player (Game|Player|GetPlayerPawn 0)))
  (Variables|Default|SetAs%20BP%20Player _asbp_player)
  (Utilities|Time|SetTimerbyEvent (delegate Custom|AIMove) 2.0 true))

(event EventHitDamage
  (params (Damage :type Float%20%28double-precision%29))
  (bind _output_get (Variables|Default|SetHealth (- (Variables|Default|GetHealth) Damage)))
  (Development|PrintString (Utilities|String|ToString(Float) _output_get))
  (if (<= _output_get 0.0)
    (CallFunction|Die)))

(event EventStun
  (params (StunAmount :type Float%20%28double-precision%29))
  (bind _charactermovement (Variables|Character|GetCharacterMovement))
  (Pawn|Components|CharacterMovement|DisableMovement _charactermovement)
  (Variables|Default|SetIsStunned true)
  (Development|PrintString "GOTSTUNTED")
  (Utilities|FlowControl|Delay StunAmount)
  (Variables|Default|SetIsStunned false)
  (Development|PrintString "free")
  (Pawn|Components|CharacterMovement|SetMovementMode _charactermovement "MOVE_Walking" 0))

(fn ConstructionScript)

(fn Die
  (bind _enemyspawner (Variables|Default|GetEnemySpawner)
    (:then
      (Default|DieMessagetoSpawner _enemyspawner)
      (Actor|DestroyActor))
    (:else)))