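; Wave spawner actor that spawns enemies at its own transform on timed triggers.
; Tick counts whole seconds and starts a wave when the count equals that wave's trigger time in a map.
; Per-wave maps set difficulty and enemy count, selecting an Easy, Medium or Hard array for random class picks.
; Spawned enemies receive a spawner reference; a death event decrements the active count, but reaching zero triggers nothing.
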(event EventDieMessagetoSpawner
  (bind _result (Math|Integer|DecrementInt (Variables|Wave|GetActiveEnemyCount))
    (:%20%20
      (if (== _result 0)
        _))))

(event EventTick
  (params (DeltaSeconds :type Float%20%28single-precision%29))
  (CallFunction|CountSeconds DeltaSeconds)
  (if (== (Variables|Default|GetCurrentTime) (.Value (Utilities|Map|Find (Variables|Wave|GetWaveTriggers) (Variables|Wave|GetCurrentWave))))
    (CallFunction|StartWave)))

(fn ConstructionScript)

(fn GetWaveHardnessandEnemyCount
  (params (Wave :type Integer%20%28by%20ref%29))
  (return (.Value (Utilities|Map|Find (Variables|Wave|GetWaveHardness) Wave)) (.Value (Utilities|Map|Find (Variables|Wave|GetWaveEnemyCount) Wave))))

(fn StartWave
  (bind _returnvalue (Transformation|GetActorTransform))
  (bind _currentwave (Variables|Wave|GetCurrentWave))
  (bind (_hardness _enemycount) (CallFunction|GetWaveHardnessandEnemyCount _currentwave))
  (Development|PrintString (Utilities|String|Append "Starting Wave" (Utilities|String|ToString(Integer) (Variables|Wave|GetCurrentWave))))
  (switch Utilities|FlowControl|Switch|SwitchonEnum_Hardness _hardness
    (:NewEnumerator0
      (Development|PrintString "easy" true true "(R=0.000000,G=0.161832,B=1.000000,A=1.000000)")
      (CallFunction|SpawnEnemies _enemycount (Variables|EnemyTypes|GetEasyEnemies) _returnvalue))
    (:NewEnumerator1
      (Development|PrintString "medim" true true "(R=0.000000,G=0.161832,B=1.000000,A=1.000000)")
      (CallFunction|SpawnEnemies _enemycount (Variables|EnemyTypes|GetMediumEnemies) _returnvalue))
    (:NewEnumerator2
      (Development|PrintString "hard" true true "(R=0.000000,G=0.161832,B=1.000000,A=1.000000)")
      (CallFunction|SpawnEnemies _enemycount (Variables|EnemyTypes|GetHardEnemies) _returnvalue)))
  (Math|Integer|IncrementInt (Variables|Wave|GetCurrentWave)))

(fn SpawnEnemies
  (params (EnemyCount :type Integer) (Array :type Array%20of%20BP%20Enemy%20Class%20References) (SpawnTransform :type Transform))
  (bind _outitem (Utilities|Array|Random Array))
  (for _index (range 1 EnemyCount)
    (if (Utilities|IsValidClass _outitem)
      (bind _returnvalue (Game|SpawnActorfromClass _outitem SpawnTransform "Undefined" "MultiplyWithRoot" 0 0))
      (Variables|/Game/Blueprints/BP_Enemy.BP_Enemy_C|SetEnemySpawner _returnvalue self)
      (Math|Integer|IncrementInt (Variables|Wave|GetActiveEnemyCount))
      (else
        (return))))
  (return))

(fn CountSeconds
  (params (DeltaTime :type Float%20%28double-precision%29))
  (bind _output_get (Variables|Default|SetAccumulatedTime (+ DeltaTime (Variables|Default|GetAccumulatedTime))))
  (if (>= _output_get 1.0)
    (Variables|Default|SetAccumulatedTime (- (Variables|Default|GetAccumulatedTime) 1.0))
    (Math|Integer|IncrementInt (Variables|Default|GetCurrentTime)
      (:%20%20
        (return)))))