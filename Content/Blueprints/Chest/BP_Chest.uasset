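; BP_Chest is a chest that offers a choice of three pickups: garlic, throwing spell and stun.
; OpenChest plays a sound and spawns the pickups once at component locations, giving each a reference back to the chest.
; ChestDestroy notifies the cached BP_GameController, then uses the picked actor's tag to destroy the other two pickups and the chest itself.
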(event EventBeginPlay
  (bind _returnvalue (Actor|GetActorOfClass "/Game/Blueprints/GameController/BP_GameController.BP_GameController_C"))
  (Variables|Default|SetGameController _returnvalue))

(event EventOpenChest
  (Audio|PlaySound2D "/Game/Sounds/S_Chest.S_Chest" 1.0 1.0 0.0 0 0)
  (CallFunction|CreatePickups))

(event EventChestDestroy
  (params (Actor :type Actor%20Object%20Reference))
  (CallFunction|Destroy Actor))

(fn ConstructionScript)

(fn CreatePickups
  (if (not (Variables|Default|GetItemsCreated))
    (bind _returnvalue (Game|SpawnActorfromClass "/Game/Blueprints/AdditionalSkills/BP_Garlic.BP_Garlic_C" (Math|Conversions|ToTransform(Vector) (Transformation|GetWorldLocation (Variables|Default|GetGarlicLoc_0))) "Undefined" "MultiplyWithRoot" 0 0))
    (Variables|Default|SetGarlic _returnvalue)
    (Variables|/Game/Blueprints/AdditionalSkills/BP_Garlic.BP_Garlic_C|SetChest _returnvalue self)
    (bind _returnvalue_2 (Game|SpawnActorfromClass "/Game/Blueprints/AdditionalSkills/ThrowingSpell/BP_ThrowingSpell.BP_ThrowingSpell_C" (Math|Conversions|ToTransform(Vector) (Transformation|GetWorldLocation (Variables|Default|GetSpellLoc))) "Undefined" "MultiplyWithRoot" 0 0))
    (Variables|Default|SetSpell _returnvalue_2)
    (Variables|/Game/Blueprints/AdditionalSkills/ThrowingSpell/BP_ThrowingSpell.BP_ThrowingSpell_C|SetChest _returnvalue_2 self)
    (bind _returnvalue_3 (Game|SpawnActorfromClass "/Game/Blueprints/AdditionalSkills/BP_StunEnemy.BP_StunEnemy_C" (Math|Conversions|ToTransform(Vector) (Transformation|GetWorldLocation (Variables|Default|GetStunLoc))) "Undefined" "MultiplyWithRoot" 0 0))
    (Variables|Default|SetZap _returnvalue_3)
    (Variables|/Game/Blueprints/AdditionalSkills/BP_StunEnemy.BP_StunEnemy_C|SetChest _returnvalue_3 self)
    (Variables|Default|SetItemsCreated true)
    (return)))

(fn Destroy
  (params (PickedActor :type Actor%20Object%20Reference))
  (Class|BPIMessager|ChestDestroy(Message) (Variables|Default|GetGameController))
  (if (Actor|ActorHasTag PickedActor "Stun")
    (Actor|DestroyActor (Variables|Default|GetSpell))
    (Actor|DestroyActor (Variables|Default|GetGarlic))
    (Actor|DestroyActor)
    (elif (Actor|ActorHasTag PickedActor "Garlic")
      (Actor|DestroyActor (Variables|Default|GetZap))
      (Actor|DestroyActor (Variables|Default|GetSpell))
      (Actor|DestroyActor)
      (elif (Actor|ActorHasTag PickedActor "ThrowSpell")
        (Actor|DestroyActor (Variables|Default|GetZap))
        (Actor|DestroyActor (Variables|Default|GetGarlic))
        (Actor|DestroyActor)))))